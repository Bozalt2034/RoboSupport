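; Player robot character that drives, grabs and rotates physics objects, and solves puzzles on a draining battery.
; Camera traces drive interaction prompts and BPI_Interact handling; puzzles switch the view and open a tool-based action widget.
; Tick updates battery, HUD, held object and custom-depth puzzle hover outlines.
; An empty battery switches the HUD screen, and GoToCharge refills it at BasePoint.
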(event `Key|H`
  (params (Key :type "Key Structure"))
  (bind _mainwidget (`self.MainWidget`))
  (:`Pressed`
    ;[1 1 1] Вызов меню подсказки
    (`/Engine/EditorBlueprintResources/StandardMacros.FlipFlop`
      (:`A`
        (`/Game/RoboSupport/UI/WBP_UiMain.HelpNotesVisibility` _mainwidget "Visible"))
      (:`B`
        (`/Game/RoboSupport/UI/WBP_UiMain.HelpNotesVisibility` _mainwidget "Hidden")))))

(event `self.ReceiveBeginPlay`
  (`self.UpdateActionList`)
  (bind _returnvalue (`|CreateWidget` "/Game/RoboSupport/UI/WBP_UiMain.WBP_UiMain_C"))
  (bind _output_get (set `self.MainWidget` _returnvalue))
  (`UserWidget.AddToViewport` _output_get 0))

(event `self.ReceiveTick`
  (params (DeltaSeconds :type "Float (single-precision)"))
  (bind _camera (`self.Camera`))
  (bind (_hitresult _returnvalue) (`PlayerController.GetHitResultUnderCursorByChannel` (`GameplayStatics.GetPlayerController` 0) "TraceTypeQuery1" true))
  (bind (_bblockinghit _binitialoverlap _time _distance _location _impactpoint _normal _impactnormal _physmat _hitactor _hitcomponent) (`GameplayStatics.BreakHitResult` _hitresult))
  (set `self.Delta Seconds` DeltaSeconds)
  (`|ExecutionSequence`
    (:`then_0`
      ;[1 1 1] Отображение плашки взаимодействие с объектом
      (`self.InteractScaner`))
    (:`then_1`
      ;[1 1 1] Разряд батареи
      (bind _batterychargelvl (`self.BatteryPassiveDischarge`))
      (`KismetSystemLibrary.PrintString` (`KismetStringLibrary.Concat_StrStr` "Charge: " (`KismetStringLibrary.Conv_DoubleToString` _batterychargelvl)) true true (struct :`G` 0.66 :`B` 1.0 :`A` 1.0) 0.0)
      (`KismetSystemLibrary.PrintString` (`KismetStringLibrary.Concat_StrStr` "Consumption: " (`KismetStringLibrary.Conv_DoubleToString` (`self.Battery_Consumption`))) true true (struct :`G` 0.66 :`B` 1.0 :`A` 1.0) 0.0)
      ;[1 1 1] Отображение заряда батареи в виджете
      (`/Game/RoboSupport/UI/WBP_Battery.Update Battery` (`/Game/RoboSupport/UI/WBP_UiMain.WBP_Battery` (`self.MainWidget`)) (`self.Battery_CurentCharge`) (`self.Battery_MaxCharge`)))
    (:`then_2`
      ;[1 1 1] Выделение элементов головоломки
      (if _returnvalue
        (bind _asbp_puzzle_base (cast `/Game/RoboSupport/Puzzle/BP_PuzzleBase` _hitactor))
        (bind _asstatic_mesh_component (cast `StaticMeshComponent` _hitcomponent))
        ;;[1 1 1] Сравнение выделяемых компонентов. Запись нового компонета впеременную, если он не равен ранее записанному.
        ;; Если равен записанному, запустить логику выделения объекта
        (if (== (`self.OverlinedComponent`) _hitcomponent)
          ;;[1 1 1] Отключение обводки
          (add `PrimitiveComponent.OnEndCursorOver` (`self.OverlinedComponent`) (delegate `OnEndCursorOver_Event_0`))
          (else
            (bind _output_get (set `self.OverlinedComponent` _asstatic_mesh_component))
            ;;[1 1 1] Определяем тело головоломки, сравнивая с записанным компонентом. Его выделять не нужно
            (if (!= (`/Game/RoboSupport/Puzzle/BP_PuzzleBase.Body` _asbp_puzzle_base) (`self.OverlinedComponent`))
              ;;[1 1 1] Включение обводки
              (add `PrimitiveComponent.OnBeginCursorOver` _output_get (delegate `OnBeginCursorOver_Event_0`)))))))
    (:`then_3`
      (if (`self.IsGrabed`)
        (`PhysicsHandleComponent.SetTargetLocation` (`self.PhysicsHandle`) (+ (* (`SceneComponent.GetForwardVector` _camera) 150.0) (`SceneComponent.K2_GetComponentLocation` _camera)))
        ;[1 1 1] Вращение схваченного объекта
        (`PhysicsHandleComponent.SetTargetRotation` (`self.PhysicsHandle`) (`KismetMathLibrary.MakeRotator` 0.0 0.0 (stale `InputAxisKey|MouseWheelAxis` _output_get)))))
    (:`then_4`
      (if (`self.Charge!0`)
        (`/Game/RoboSupport/UI/WBP_UiMain.SwitchScreen` (`self.MainWidget`) 0)
        (else
          (`/Game/RoboSupport/UI/WBP_UiMain.SwitchScreen` (`self.MainWidget`) 1)
          (set `PlayerController.bShowMouseCursor` true (`GameplayStatics.GetPlayerController` 0)))))))

(event `InputAxisKey|MouseWheelAxis`
  (params (AxisValue :type "Float (single-precision)"))
  ;[1 1 1] Вращение схваченного объекта
  ;;[1 1 1] Вычисление поворота модели
  (bind _output_get (set `self.RotationGrabetObject` (+ (`self.RotationGrabetObject`) (* AxisValue 10.0)))))

(event `GoToCharge`
  (set `self.Battery_CurentCharge` 100.0)
  (`self.K2_SetActorLocation` (`self.K2_GetActorLocation` (`self.BasePoint`)))
  (set `PlayerController.bShowMouseCursor` false (`GameplayStatics.GetPlayerController` 0)))

(event `OnClicked_Event_0`
  (params (TouchedComponent :type "PrimitiveComponent Object Reference") (ButtonPressed :type "Key Structure" :default "None"))
  ;[1 0.2795 0] TEstZone
  (`KismetSystemLibrary.PrintString` "Hello" true true (struct :`R` 1.0 :`A` 1.0)))

(event `InputAxis|MoveForward`
  (params (AxisValue :type "Float (single-precision)"))
  ;[1 1 1] Move Forward/Backward
  (`self.K2_AddActorLocalOffset` (`KismetMathLibrary.MakeVector` (* AxisValue (`self.ForwardSpeed`)))))

(event `CustomEvent_0`
  (params (TouchedComponent :type "PrimitiveComponent Object Reference") (ButtonPressed :type "Key Structure" :default "None"))
  ;[1 0.2795 0] TEstZone
)

(event `Key|G`
  (params (Key :type "Key Structure"))
  (bind _camera (`self.Camera`))
  (bind _returnvalue (`SceneComponent.K2_GetComponentLocation` _camera))
  (:`Pressed`
    ;[1 1 1] Grab system
    (if (`self.IsGrabed`)
      (`PhysicsHandleComponent.ReleaseComponent` (`self.PhysicsHandle`))
      (set `self.IsGrabed` false)
      (set `self.RotationGrabetObject` 0.0)
      (else
        (bind (_outhit _returnvalue_2) (`KismetSystemLibrary.LineTraceSingle` :`Start` _returnvalue :`End` (+ (* (`SceneComponent.GetForwardVector` _camera) 250.0) _returnvalue) :`TraceChannel` "TraceTypeQuery1" :`DrawDebugType` "ForDuration"))
        (if _returnvalue_2
          (bind (_bblockinghit _binitialoverlap _time _distance _location _impactpoint _normal _impactnormal _physmat _hitactor _hitcomponent) (`GameplayStatics.BreakHitResult` _outhit))
          (`PhysicsHandleComponent.GrabComponentAtLocationWithRotation` :`self` (`self.PhysicsHandle`) :`Component` _hitcomponent :`Location` (`SceneComponent.K2_GetComponentLocation` _hitcomponent))
          (set `self.IsGrabed` true))))))

(event `InputAxis|MoveRight`
  (params (AxisValue :type "Float (single-precision)"))
  ;[1 1 1] Move Right/Left
  (`self.K2_AddActorLocalRotation` (`KismetMathLibrary.MakeRotator` 0.0 0.0 (* AxisValue (`self.TurnSpeed`)))))

(event `Key|LeftMouseButton`
  (params (Key :type "Key Structure"))
  ;[1 0.2795 0] TEstZone
  (:`Pressed`
    (bind _asbp_puzzle_comp (cast `/Game/RoboSupport/Puzzle/BP_PuzzleComp` (`.HitActor` (`GameplayStatics.BreakHitResult` (`PlayerController.GetHitResultUnderCursorForObjects` (cast `PlayerController` (`self.GetController`) :!pure true) (`|MakeArray` "ObjectTypeQuery2" :!type "EObjectTypeQuery Enum") true)))))))

(event `InputAxis|Turn`
  (params (AxisValue :type "Float (single-precision)"))
  ;[1 1 1] Rotate view
  (`SceneComponent.K2_AddLocalRotation` (`self.Head`) (`KismetMathLibrary.MakeRotator` 0.0 0.0 AxisValue) false false))

(event `InputAxis|Up`
  (params (AxisValue :type "Float (single-precision)"))
  ;[1 1 1] Rise/lower view
  (`SceneComponent.K2_AddLocalRotation` (`self.Camera`) (`KismetMathLibrary.MakeRotator` 0.0 AxisValue) false false))

(event `Key|LeftMouseButton`
  (params (Key :type "Key Structure"))
  ;[1 0.2795 0] TEstZone
)

(event `Key|L`
  (params (Key :type "Key Structure"))
  ;[1 0.2795 0] TEstZone
  (:`Pressed`
    (for _array_element (`/Game/RoboSupport/Inventory/AC_InventoriComponent.Inventory` (`self.BPC_InventoriComponent`))
      (bind (_name _amount _index _type _itemclass) (break `/Game/RoboSupport/Inventory/BPS_ItemStructure` _array_element))
      (if (!= _itemclass null)
        (`KismetSystemLibrary.PrintString` (`KismetStringLibrary.Concat_StrStr` (`KismetTextLibrary.Conv_TextToString` _name) (`KismetStringLibrary.Conv_IntToString` _amount)))))))

(event `InputAction|Interact`
  (params (Key :type "Key Structure"))
  ;[1 1 1] Interaction
  (:`Pressed`
    (`self.InteractionSystem`)))

(event `Key|Three`
  (params (Key :type "Key Structure"))
  ;[1 1 1] Test battery discharge
  (:`Pressed`
    (`self.Battery Disсharge` 50.0)))

(event `Key|Two`
  (params (Key :type "Key Structure"))
  ;[1 1 1] Test battery charge
  (:`Pressed`
    (`self.Battery Charge` 10.0)))

(event `OnEndCursorOver_Event_0`
  (params (TouchedComponent :type "PrimitiveComponent Object Reference"))
  ;[1 1 1] Выделение элементов головоломки
  ;;[1 1 1] Отключение обводки
  (`PrimitiveComponent.SetRenderCustomDepth` TouchedComponent false))

(event `Key|One`
  (params (Key :type "Key Structure"))
  (:`Pressed`
    (`self.AddTools` "NewEnumerator3")))

(event `Key|K`
  (params (Key :type "Key Structure"))
  ;[1 0.6767 0] Тест ui
  (:`Pressed`
    (bind _activewidget (`self.ActiveWidget`)
      (:`then`
        (`Widget.RemoveFromParent` _activewidget)
        (set `self.ActiveWidget` null)
        (set `PlayerController.bShowMouseCursor` false (`GameplayStatics.GetPlayerController` 0)))
      (:`else`
        (bind _returnvalue (`|CreateWidget` "/Game/RoboSupport/UI/Puzzle/WBP_PuzzleElemBase.WBP_PuzzleElemBase_C"))
        (bind _output_get (set `self.ActiveWidget` _returnvalue))
        (`UserWidget.AddToViewport` _output_get 0)))))

(event `OnBeginCursorOver_Event_0`
  (params (TouchedComponent :type "PrimitiveComponent Object Reference"))
  ;[1 1 1] Выделение элементов головоломки
  ;;[1 1 1] Включение обводки
  (`PrimitiveComponent.SetRenderCustomDepth` TouchedComponent true))

(fn `AddCart`
  (params (Interactor :type "Actor Object Reference"))
  (returns (NewParam :type Boolean))
  (return false))

(fn `AddTools`
  (params (NewItem :type "/Game/RoboSupport/Inventory/E_Tools Enum" :default "NewEnumerator1"))
  (`KismetArrayLibrary.Array_AddUnique` (`self.MyTools`) NewItem)
  (`self.UpdateActionList`))

(fn `Battery Charge`
  (params (B :type "Float (double-precision)"))
  (bind _battery_curentcharge (`self.Battery_CurentCharge`))
  (set `self.Battery_CurentCharge` (+ _battery_curentcharge B))
  (if (>= _battery_curentcharge 100.0)
    (set `self.Battery_CurentCharge` 100.0)))

(fn `Battery Disсharge`
  (params (Discharge :type "Float (double-precision)"))
  (if (>= (`self.Battery_CurentCharge`) 0.0)
    (set `self.Battery_CurentCharge` (- (`self.Battery_CurentCharge`) Discharge))))

(fn `BatteryPassiveDischarge`
  (returns (BatteryChargeLvl :type "Float (double-precision)"))
  ;[1 1 1] Расход батареи
  ;;[1 1 1] Проверяем уровень заряда
  (if (>= (`self.Battery_CurentCharge`) 0.01)
    (set `self.Charge!0` true)
    ;;[1 1 1] Установка расхода заряда по статусу: двигается/не двигается
    (if (or (!= (`self.GetInputAxisValue`) 0.0) (!= (`self.GetInputAxisValue`) 0.0))
      (set `self.Battery_Consumption` (`self.Battery_InMoveConsumption`))
      (else
        (set `self.Battery_Consumption` (`self.Battery_PaasiveConsumption`))))
    ;;[1 1 1] Вычетание заряда аккумулятора
    (bind _output_get (set `self.Battery_CurentCharge` (`KismetMathLibrary.FInterpTo_Constant` (`self.Battery_CurentCharge`) 0.0 (`self.Delta Seconds`) (/ (`self.Battery_Consumption`) (`self.Battery_ConsumptionTime`)))))
    (return _output_get)
    (else
      ;;[1 1 1] Установка переменной наличия заряда на лож
      (set `self.Battery_CurentCharge` 0.0)
      (set `self.Charge!0` false))))

(fn `CreatePuzzleUi`
  (params (Actions :type "Map of /Game/RoboSupport/Inventory/E_Tools Enum to String") (InteractObject :type "Actor Object Reference") (PuzzleRef :type "/Game/RoboSupport/Puzzle/BP_PuzzleBase Object Reference"))
  (locals (Ref :type "/Game/RoboSupport/Puzzle/BP_PuzzleBase Object Reference"))
  (bind _activewidget (`self.ActiveWidget`)
    (:`then`
      (`Widget.RemoveFromParent` _activewidget)
      (set `self.ActiveWidget` null)
      (set `PlayerController.bShowMouseCursor` false (`GameplayStatics.GetPlayerController` 0)))
    (:`else`
      (bind _returnvalue (`|CreateWidget` "/Game/RoboSupport/UI/Puzzle/WBP_PuzzleElemBase.WBP_PuzzleElemBase_C"))
      (bind _output_get (set `self.ActiveWidget` _returnvalue))
      (`UserWidget.AddToViewport` _output_get 0)
      (`/Game/RoboSupport/UI/Puzzle/WBP_UiElem1.FillData` (`/Game/RoboSupport/UI/Puzzle/WBP_PuzzleElemBase.WBP_UiElem1` (`self.ActiveWidget`)) (`self.MyTools`) (`local.Actions`) InteractObject)
      (`self.UpdatePuzzleProblems` InteractObject)
      (set `PlayerController.bShowMouseCursor` true (`GameplayStatics.GetPlayerController` 0)))))

(fn `Interact`
  (params (Interactor :type "Actor Object Reference"))
  (return))

(fn `InteractionSystem`
  (locals (InteractActor :type "Actor Object Reference"))
  (bind _returnvalue (`GameplayStatics.GetPlayerController` 0))
  (bind _camera (`self.Camera`))
  (bind _returnvalue_2 (`SceneComponent.K2_GetComponentLocation` _camera))
  (`|ExecutionSequence`
    (:`then_0`
      (bind (_outhit _returnvalue_3) (`KismetSystemLibrary.SphereTraceSingle` :`Start` _returnvalue_2 :`End` (+ (* (`SceneComponent.GetForwardVector` _camera) 250.0) _returnvalue_2) :`Radius` 10.0 :`TraceChannel` "TraceTypeQuery1" :`DrawDebugType` "ForDuration"))
      (if _returnvalue_3
        (bind _output_get (set `self.HitResult` _outhit))
        (bind (_bblockinghit _binitialoverlap _time _distance _location _impactpoint _normal _impactnormal _physmat _hitactor) (`GameplayStatics.BreakHitResult` _output_get))
        (set `local.InteractActor` _hitactor)
        (bind _newparam (message `/Game/RoboSupport/Interface/BPI_Interact.GetInteractableType` _hitactor))
        (message `/Game/RoboSupport/Interface/BPI_Interact.SetInteractor` _hitactor self)
        (switch `/Game/RoboSupport/Objects/E_InteractType` _newparam
          (:`NewEnumerator0`
            (message `/Game/RoboSupport/Interface/BPI_Interact.Interact` (`local.InteractActor`) self "NewEnumerator1" "NewEnumerator0")
            (`self.Battery Disсharge` (`self.InteractDischarge`)))
          (:`NewEnumerator1`
            (bind (_actions _puzzleref) (message `/Game/RoboSupport/Interface/BPI_Interact.GetInteractableActions` _hitactor))
            (`self.CreatePuzzleUi` _actions (`local.InteractActor`))
            ;[1 1 1] Переключение камеры на головоломку
            (`PlayerController.SetViewTargetWithBlend` (`GameplayStatics.GetPlayerController` 0) _puzzleref 0.0 "VTBlend_Linear" 0.0 false)
            ;[1 1 1] Включение ивентов клик и наведение курсора
            (set `PlayerController.bEnableClickEvents` true _returnvalue)
            (set `PlayerController.bEnableMouseOverEvents` true _returnvalue)
            ;[1 1 1] Не отключает переиещение и обзор персонажа
            ;;[1 1 1] Отключение инпутов персонажа
            (`Controller.SetIgnoreLookInput` _returnvalue true)
            (`Controller.SetIgnoreMoveInput` _returnvalue true)
            (set `PlayerController.bShowMouseCursor` true _returnvalue))
          (:`NewEnumerator2`
            (message `/Game/RoboSupport/Interface/BPI_Interact.Interact` (`local.InteractActor`) self "NewEnumerator1" "NewEnumerator0")))))
    (:`then_1`
      (`local.InteractActor`
        (:`then`
          (bind _asbp_puzzle_base (cast `/Game/RoboSupport/Puzzle/BP_PuzzleBase` (`local.InteractActor`)))
          (add `/Game/RoboSupport/Puzzle/BP_PuzzleBase.OnUpdateState` _asbp_puzzle_base (`|CreateDelegate` :!event `Puzzle Update`)))
        (:`else`)))))

(fn `InteractScaner`
  (bind _mainwidget (`self.MainWidget`))
  (bind _camera (`self.Camera`))
  (bind _mainwidget_2 (`self.MainWidget`))
  (bind _returnvalue (`SceneComponent.K2_GetComponentLocation` _camera))
  (bind _returnvalue_2 (`Widget.IsVisible` (`/Game/RoboSupport/UI/WBP_UiMain.B_interactE` (`self.MainWidget`))))
  (bind _returnvalue_3 (`Widget.IsVisible` (`/Game/RoboSupport/UI/WBP_UiMain.B_interactE` (`self.MainWidget`))))
  (`self.MainWidget`
    (:`then`
      (bind (_outhit _returnvalue_4) (`KismetSystemLibrary.LineTraceSingle` _returnvalue (+ (* (`SceneComponent.GetForwardVector` _camera) 250.0) _returnvalue) "TraceTypeQuery1"))
      (if _returnvalue_4
        (bind (_bblockinghit _binitialoverlap _time _distance _location _impactpoint _normal _impactnormal _physmat _hitactor) (`GameplayStatics.BreakHitResult` _outhit))
        (bind _newparam (message `/Game/RoboSupport/Interface/BPI_Interact.GetInteractableType` _hitactor))
        (switch `/Game/RoboSupport/Objects/E_InteractType` _newparam
          (:`NewEnumerator0`
            (bind _returnvalue_5 (`KismetSystemLibrary.DoesImplementInterface` _hitactor "/Game/RoboSupport/Interface/BPI_Interact.BPI_Interact_C"))
            (if _returnvalue_5 :!label _label
              (if (not _returnvalue_2)
                (`/Game/RoboSupport/UI/WBP_UiMain.UpdateInteract` _mainwidget "Visible" "E для взаимодействия"))
              (else
                (if _returnvalue_2 :!label _label_2
                  (`/Game/RoboSupport/UI/WBP_UiMain.UpdateInteract` _mainwidget "Hidden" "E для взаимодействия")))))
          (:`NewEnumerator1`
            (goto _label))
          (:`NewEnumerator3`
            (if _returnvalue_5
              (if (not _returnvalue_3)
                (`/Game/RoboSupport/UI/WBP_UiMain.UpdateInteract` _mainwidget_2 "Visible" "G поднять/отпустить"))
              (elif _returnvalue_3
                (`/Game/RoboSupport/UI/WBP_UiMain.UpdateInteract` _mainwidget_2 "Hidden" "G поднять/отпустить")))))
        (else
          (goto _label_2))))
    (:`else`)))

(fn `Puzzle Update`
  (params (PuzzleBaseObject :type "/Game/RoboSupport/Puzzle/BP_PuzzleBase Object Reference"))
  (`self.UpdatePuzzleProblems` PuzzleBaseObject))

(fn `PuzzleInteract`
  (params (NewParam1 :type "Actor Object Reference"))
  (returns (NewParam :type "/Game/RoboSupport/Characters/BP_RobotSupport Object Reference"))
  (return null))

(fn `RemoveTools`
  (params (Item :type "/Game/RoboSupport/Inventory/E_Tools Enum" :default "NewEnumerator1"))
  (`KismetArrayLibrary.Array_RemoveItem` (`self.MyTools`) Item)
  (`self.UpdateActionList`))

(fn `Update Puzzle State`)

(fn `UpdateActionList`
  (`KismetArrayLibrary.Array_Clear` (`self.MyActionList`))
  (for _array_element (`self.MyTools`)
    (`KismetArrayLibrary.Array_Add` (`self.MyActionList`) (`|GetEnumeratorNameAsString` _array_element))))

(fn `UpdatePuzzleProblems`
  (params (Object :type "Object Object Reference"))
  (bind _wbp_puzzledescription (`/Game/RoboSupport/UI/Puzzle/WBP_PuzzleElemBase.WBP_PuzzleDescription` (`self.ActiveWidget`)))
  ;[1 1 1] Получение текста ошибки из головоломки
  (bind _asbp_puzzle_base (cast `/Game/RoboSupport/Puzzle/BP_PuzzleBase` Object))
  (for _array_element (`/Game/RoboSupport/Puzzle/BP_PuzzleBase.Problems` _asbp_puzzle_base)
    (bind (_name _defectstatus) (break `/Game/RoboSupport/Puzzle/F_defects` _array_element))
    ;[1 1 1] Заполняем виджет описания текстом
    (`/Game/RoboSupport/UI/Puzzle/WBP_PuzzleDescription.Fill Text` _wbp_puzzledescription _name _defectstatus)
    ;[1 1 1] Заполняем заголовок задачи
    (`/Game/RoboSupport/UI/Puzzle/WBP_PuzzleDescription.SetHeaderText` _wbp_puzzledescription (`/Game/RoboSupport/Puzzle/BP_PuzzleBase.ProblemHeader` _asbp_puzzle_base))))

(fn `UserConstructionScript`)