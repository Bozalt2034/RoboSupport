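; Accountant NPC that, on interaction, checks the player's tasks: getting the office worker's report and connecting the PC mouse.
; Interact looks up both task items in the interactor's inventory, using a short Delay on the first Sequence branch so both flags update before branching.
; Success adds ItemToAdd to the player robot's inventory; each outcome shows a timed WBP_WarningText.
; The combined-task warning is unreachable, and other interaction functions return defaults.
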(event `/Game/RoboSupport/Interface/BPI_Interact.Interact`
  (params (Interactor :type "Actor Object Reference") (CurrentTool :type "/Game/RoboSupport/Inventory/E_Tools Enum" :default "NewEnumerator4") (PbutoonAct :type "/Game/RoboSupport/Puzzle/E_ElemPButtonAct Enum" :default "NewEnumerator0"))
  (bind _returnvalue (`self.K2_GetComponentsByClass` Interactor "/Game/RoboSupport/Inventory/AC_InventoriComponent.AC_InventoriComponent_C"))
  (`|ExecutionSequence`
    (:`then_0`
      (`KismetSystemLibrary.Delay` 0.2)
      (if (`self.HaveReport`)
        (if (`self.HavBookkipingPCFix`)
          (if (and (`self.HaveReport`) (`self.HavBookkipingPCFix`))
            (bind _asbp_robot_support (cast `/Game/RoboSupport/Characters/BP_RobotSupport` (`GameplayStatics.GetPlayerPawn` 0)))
            (`/Game/RoboSupport/Inventory/AC_InventoriComponent.AddItem` (`/Game/RoboSupport/Characters/BP_RobotSupport.BPC_InventoriComponent` _asbp_robot_support) (`self.ItemToAdd`))
            (bind _returnvalue_2 (`|CreateWidget` "/Game/RoboSupport/Objects/Widget/WBP_WarningText.WBP_WarningText_C" (`GameplayStatics.GetPlayerController` 0) "Задание бухгалтера выполнено" (struct :`R` 0.02952 :`G` 1.0 :`A` 1.0)))
            (bind _output_get (set `self.ActiveWidget` _returnvalue_2))
            (`UserWidget.AddToViewport` _output_get 0)
            (`KismetSystemLibrary.Delay` 3.0)
            (`Widget.RemoveFromParent` (`self.ActiveWidget`))
            (else
              (bind _returnvalue_3 (`|CreateWidget` "/Game/RoboSupport/Objects/Widget/WBP_WarningText.WBP_WarningText_C" (`GameplayStatics.GetPlayerController` 0) "Выполнить задачи: \n- Получить отчет офисного работника \n- Подключить мышку к ПК" (struct :`R` 1.0 :`A` 1.0)))
              (bind _output_get_2 (set `self.ActiveWidget` _returnvalue_3))
              (`UserWidget.AddToViewport` _output_get_2 0)
              (`KismetSystemLibrary.Delay` 3.0)
              (`Widget.RemoveFromParent` (`self.ActiveWidget`))))
          (else
            (bind _returnvalue_4 (`|CreateWidget` "/Game/RoboSupport/Objects/Widget/WBP_WarningText.WBP_WarningText_C" (`GameplayStatics.GetPlayerController` 0) "Выполнить задачи: \n- Подключить мышку к ПК" (struct :`R` 1.0 :`A` 1.0)))
            (bind _output_get_3 (set `self.ActiveWidget` _returnvalue_4))
            (`UserWidget.AddToViewport` _output_get_3 0)
            (`KismetSystemLibrary.Delay` 3.0)
            (`Widget.RemoveFromParent` (`self.ActiveWidget`))))
        (else
          (bind _returnvalue_5 (`|CreateWidget` "/Game/RoboSupport/Objects/Widget/WBP_WarningText.WBP_WarningText_C" (`GameplayStatics.GetPlayerController` 0) "Выполнить задачи: \n- Получить отчет офисного работника" (struct :`R` 1.0 :`A` 1.0)))
          (bind _output_get_4 (set `self.ActiveWidget` _returnvalue_5))
          (`UserWidget.AddToViewport` _output_get_4 0)
          (`KismetSystemLibrary.Delay` 3.0)
          (`Widget.RemoveFromParent` (`self.ActiveWidget`)))))
    (:`then_1`
      (bind _success (`/Game/RoboSupport/Inventory/AC_InventoriComponent.FindeItem` _returnvalue (make `/Game/RoboSupport/Inventory/BPS_ItemStructure` "" 0 0 "NewEnumerator11")))
      (set `self.HaveReport` _success))
    (:`then_2`
      (bind _success_2 (`/Game/RoboSupport/Inventory/AC_InventoriComponent.FindeItem` _returnvalue (make `/Game/RoboSupport/Inventory/BPS_ItemStructure` "" 0 0 "NewEnumerator13")))
      (set `self.HavBookkipingPCFix` _success_2))))

(fn `AddCart`
  (params (Interactor :type "Actor Object Reference"))
  (returns (NewParam :type Boolean))
  (return false))

(fn `GetInteractableActions`
  (returns (Actions :type "Map of /Game/RoboSupport/Inventory/E_Tools Enum to String") (PuzzleRef :type "Actor Object Reference"))
  (return _ null))

(fn `GetInteractableType`
  (returns (NewParam :type "/Game/RoboSupport/Objects/E_InteractType Enum"))
  (return "NewEnumerator0"))

(fn `PuzzleInteract`
  (params (AnyTextIn :type String))
  (returns (AnyTextOut :type String))
  (return ""))

(fn `UserConstructionScript`)