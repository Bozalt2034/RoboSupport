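; BP_Boss is an interactable boss NPC that grants yellow access once the player has helped the bookkeeper.
; Interact searches the interactor's inventory for a specific item type and, if found, adds ItemToAdd to player 0's BP_RobotSupport inventory, without removing the checked item or guarding against repeats.
; Either branch shows a three-second WBP_WarningText: yellow confirmation or red task reminder.
; The other interaction functions return only defaults.
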(event `/Game/RoboSupport/Interface/BPI_Interact.Interact`
  (params (Interactor :type "Actor Object Reference") (CurrentTool :type "/Game/RoboSupport/Inventory/E_Tools Enum" :default "NewEnumerator4") (PbutoonAct :type "/Game/RoboSupport/Puzzle/E_ElemPButtonAct Enum" :default "NewEnumerator0"))
  (bind _success (`/Game/RoboSupport/Inventory/AC_InventoriComponent.FindeItem` (`self.K2_GetComponentsByClass` Interactor "/Game/RoboSupport/Inventory/AC_InventoriComponent.AC_InventoriComponent_C") (make `/Game/RoboSupport/Inventory/BPS_ItemStructure` "" 0 0 "NewEnumerator12")))
  (set `self.HavBookkip` _success)
  (if (`self.HavBookkip`)
    (bind _asbp_robot_support (cast `/Game/RoboSupport/Characters/BP_RobotSupport` (`GameplayStatics.GetPlayerPawn` 0)))
    (`/Game/RoboSupport/Inventory/AC_InventoriComponent.AddItem` (`/Game/RoboSupport/Characters/BP_RobotSupport.BPC_InventoriComponent` _asbp_robot_support) (`self.ItemToAdd`))
    (bind _returnvalue (`|CreateWidget` "/Game/RoboSupport/Objects/Widget/WBP_WarningText.WBP_WarningText_C" (`GameplayStatics.GetPlayerController` 0) "Желтый доступ получен" (struct :`R` 1.0 :`G` 0.84129 :`A` 1.0)))
    (bind _output_get (set `self.ActiveWidget` _returnvalue))
    (`UserWidget.AddToViewport` _output_get 0)
    (`KismetSystemLibrary.Delay` 3.0)
    (`Widget.RemoveFromParent` (`self.ActiveWidget`))
    (else
      (bind _returnvalue_2 (`|CreateWidget` "/Game/RoboSupport/Objects/Widget/WBP_WarningText.WBP_WarningText_C" (`GameplayStatics.GetPlayerController` 0) "Выполнить задачу: \n- Помочь бухгалтеру" (struct :`R` 1.0 :`A` 1.0)))
      (bind _output_get_2 (set `self.ActiveWidget` _returnvalue_2))
      (`UserWidget.AddToViewport` _output_get_2 0)
      (`KismetSystemLibrary.Delay` 3.0)
      (`Widget.RemoveFromParent` (`self.ActiveWidget`)))))

(fn `AddCart`
  (params (Interactor :type "Actor Object Reference"))
  (returns (NewParam :type Boolean))
  (return false))

(fn `GetInteractableActions`
  (returns (Actions :type "Map of /Game/RoboSupport/Inventory/E_Tools Enum to String") (PuzzleRef :type "Actor Object Reference"))
  (return _ null))

(fn `GetInteractableType`
  (returns (NewParam :type "/Game/RoboSupport/Objects/E_InteractType Enum"))
  (return "NewEnumerator0"))

(fn `PuzzleInteract`
  (params (AnyTextIn :type String))
  (returns (AnyTextOut :type String))
  (return ""))

(fn `UserConstructionScript`)