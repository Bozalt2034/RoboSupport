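; Office worker NPC that gates a task chain on the interactor's inventory, warning on screen about printer paper, computer or coffee.
; Passing the first check spawns a red card on every interaction; a short delay lets coffee flags update before branching.
; Coffee type sets how quickly a report spawns, while the EDCola mix sends him screaming along a spline before his meshes are destroyed.
; His Box overlap enables physics on code doors.
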(event `/Game/RoboSupport/Interface/BPI_Interact.Interact`
  (params (Interactor :type "Actor Object Reference") (CurrentTool :type "/Game/RoboSupport/Inventory/E_Tools Enum" :default "NewEnumerator4") (PbutoonAct :type "/Game/RoboSupport/Puzzle/E_ElemPButtonAct Enum" :default "NewEnumerator0"))
  (set `self.Interactor` Interactor)
  (bind _success (`self.FindCoffee` "NewEnumerator14"))
  (if _success
    (`|SpawnActorFromClass` "/Game/RoboSupport/Inventory/Items/BP_Card_Red.BP_Card_Red_C" (`self.GetTransform` (`self.SpawnPoint`)) "Undefined" "OverrideRootScale" null null)
    (bind _success_2 (`self.FindCoffee` "NewEnumerator10"))
    (if _success_2
      (`|ExecutionSequence`
        (:`then_0`
          (`KismetSystemLibrary.Delay` 0.2)
          (if (`self.Coffe`)
            (`/Engine/EditorBlueprintResources/StandardMacros.DoOnce` false
              (:`Completed`
                (`SceneComponent.SetVisibility` (`self.TextRender`) true false)
                (`KismetSystemLibrary.Delay` 10.0)
                (`|SpawnActorFromClass` "/Game/RoboSupport/Inventory/Items/BP_OfficeReport.BP_OfficeReport_C" (`self.GetTransform` (`self.SpawnPoint`)) "Undefined" "OverrideRootScale" null null)
                (`SceneComponent.SetVisibility` (`self.TextRender`) false false)))
            (elif (or (`self.Coffe+ED`) (`self.Coffe+Cola`))
              (`/Engine/EditorBlueprintResources/StandardMacros.DoOnce` false
                (:`Completed`
                  (`SceneComponent.SetVisibility` (`self.TextRender`) true false)
                  (`KismetSystemLibrary.Delay` 3.0)
                  (`|SpawnActorFromClass` "/Game/RoboSupport/Inventory/Items/BP_OfficeReport.BP_OfficeReport_C" (`self.GetTransform` (`self.SpawnPoint`)) "Undefined" "OverrideRootScale" null null)
                  (`SceneComponent.SetVisibility` (`self.TextRender`) false false)))
              (elif (`self.Coffe+ED+Cola`)
                (`GameplayStatics.SpawnSoundAtLocation` "/Game/RoboSupport/Characters/Audio/wilhelm_scream_Cue.wilhelm_scream_Cue" (`self.K2_GetActorLocation`) (struct) 1.0 1.0 0.0 null null)
                (bind (_direction _moveactor) (`Timeline|MovingActor`)
                  (:`Update`
                    (`SceneComponent.K2_SetWorldLocation` (`self.Body`) (`SplineComponent.GetLocationAtTime` (`self.Spline`) _moveactor "World" false) false false))
                  (:`Finished`
                    (`ActorComponent.K2_DestroyComponent` (`self.Body`))
                    (`ActorComponent.K2_DestroyComponent` (`self.StaticMesh`))))
                (else
                  (bind _returnvalue (`|CreateWidget` "/Game/RoboSupport/Objects/Widget/WBP_WarningText.WBP_WarningText_C" (`GameplayStatics.GetPlayerController` 0) "Выполнить задачу: \n- Принест Кофе" (struct :`R` 1.0 :`A` 1.0)))
                  (bind _output_get (set `self.ActiveWidget` _returnvalue))
                  (`UserWidget.AddToViewport` _output_get 0)
                  (`KismetSystemLibrary.Delay` 3.0)
                  (`Widget.RemoveFromParent` (`self.ActiveWidget`)))))))
        (:`then_1`
          (bind _success_3 (`self.FindCoffee` "NewEnumerator5"))
          (set `self.Coffe` _success_3))
        (:`then_2`
          (bind _success_4 (`self.FindCoffee` "NewEnumerator7"))
          (set `self.Coffe+ED` _success_4))
        (:`then_3`
          (bind _success_5 (`self.FindCoffee` "NewEnumerator6"))
          (set `self.Coffe+Cola` _success_5))
        (:`then_4`
          (bind _success_6 (`self.FindCoffee` "NewEnumerator8"))
          (set `self.Coffe+ED+Cola` _success_6)))
      (else
        (bind _returnvalue_2 (`|CreateWidget` "/Game/RoboSupport/Objects/Widget/WBP_WarningText.WBP_WarningText_C" (`GameplayStatics.GetPlayerController` 0) "Выполнить задачу: \n- Включить компьютер" (struct :`R` 1.0 :`A` 1.0)))
        (bind _output_get_2 (set `self.ActiveWidget` _returnvalue_2))
        (`UserWidget.AddToViewport` _output_get_2 0)
        (`KismetSystemLibrary.Delay` 3.0)
        (`Widget.RemoveFromParent` (`self.ActiveWidget`))))
    (else
      (bind _returnvalue_3 (`|CreateWidget` "/Game/RoboSupport/Objects/Widget/WBP_WarningText.WBP_WarningText_C" (`GameplayStatics.GetPlayerController` 0) "Выполнить задачу: \n- Добавить бумагу в принтер" (struct :`R` 1.0 :`A` 1.0)))
      (bind _output_get_3 (set `self.ActiveWidget` _returnvalue_3))
      (`UserWidget.AddToViewport` _output_get_3 0)
      (`KismetSystemLibrary.Delay` 3.0)
      (`Widget.RemoveFromParent` (`self.ActiveWidget`)))))

(event `self.Box.OnComponentBeginOverlap`
  (params (OverlappedComponent :type "PrimitiveComponent Object Reference") (OtherActor :type "Actor Object Reference") (OtherComp :type "PrimitiveComponent Object Reference") (OtherBodyIndex :type Integer) (bFromSweep :type Boolean) (SweepResult :type "HitResult Structure (by ref)"))
  (bind _asbp_code_doore (cast `/Game/RoboSupport/Objects/BP_CodeDoore` OtherActor))
  (`PrimitiveComponent.SetSimulatePhysics` (`/Game/RoboSupport/Objects/BP_CodeDoore.Door` _asbp_code_doore) true))

(fn `AddCart`
  (params (Interactor :type "Actor Object Reference"))
  (returns (NewParam :type Boolean))
  (return false))

(fn `FindCoffee`
  (params (`Type Coffee` :type "/Game/RoboSupport/Inventory/En_ItemType Enum" :default "NewEnumerator3"))
  (returns (Success :type Boolean))
  (bind _success (`/Game/RoboSupport/Inventory/AC_InventoriComponent.FindeItem` (`self.K2_GetComponentsByClass` (`self.Interactor`) "/Game/RoboSupport/Inventory/AC_InventoriComponent.AC_InventoriComponent_C") (make `/Game/RoboSupport/Inventory/BPS_ItemStructure` "" 0 0 `Type Coffee`)))
  (return _success))

(fn `GetInteractableActions`
  (returns (Actions :type "Map of /Game/RoboSupport/Inventory/E_Tools Enum to String") (PuzzleRef :type "Actor Object Reference"))
  (return _ null))

(fn `GetInteractableType`
  (returns (NewParam :type "/Game/RoboSupport/Objects/E_InteractType Enum"))
  (return "NewEnumerator2"))

(fn `PuzzleInteract`
  (params (AnyTextIn :type String))
  (returns (AnyTextOut :type String))
  (return ""))

(fn `UserConstructionScript`)