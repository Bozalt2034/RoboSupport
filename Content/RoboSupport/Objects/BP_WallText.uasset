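; BP_WallText is an actor that shows a line of text in the level through a widget component, such as a label on a wall.
; The construction script sets the widget's draw size from a Size variable.
; On BeginPlay it casts the component's widget to WBP_WallText and passes the Text variable to it.
; An unconnected branch that would create and assign the widget at runtime never runs.
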(event `self.ReceiveBeginPlay`
  (bind _aswbp_wall_text (cast `/Game/RoboSupport/Objects/Widget/WBP_WallText` (`WidgetComponent.GetUserWidgetObject` (`self.Widget`))))
  (`/Game/RoboSupport/Objects/Widget/WBP_WallText.SetWidgetText` _aswbp_wall_text (`self.Text`)))

(fn `UserConstructionScript`
  (`WidgetComponent.SetDrawSize` (`self.Widget`) (`self.Size`)))