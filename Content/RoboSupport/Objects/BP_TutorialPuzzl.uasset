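; BP_TutorialPuzzl is an interactable tutorial puzzle object that displays configurable wall text through a widget component.
; The construction script sizes the widget, and BeginPlay passes the text to its WBP_WallText.
; Interact creates a WBP_Tutorial_Puzzle screen widget if none is active and shows the mouse cursor.
; The other interaction functions, such as AddCart and PuzzleInteract, return only default values.
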(event `self.ReceiveBeginPlay`
  (bind _aswbp_wall_text (cast `/Game/RoboSupport/Objects/Widget/WBP_WallText` (`WidgetComponent.GetUserWidgetObject` (`self.Widget`))))
  (`/Game/RoboSupport/Objects/Widget/WBP_WallText.SetWidgetText` _aswbp_wall_text (`self.Text`)))

(event `/Game/RoboSupport/Interface/BPI_Interact.Interact`
  (params (Interactor :type "Actor Object Reference") (CurrentTool :type "/Game/RoboSupport/Inventory/E_Tools Enum" :default "NewEnumerator4") (PbutoonAct :type "/Game/RoboSupport/Puzzle/E_ElemPButtonAct Enum" :default "NewEnumerator0"))
  (`self.ActivWidget`
    (:`then`)
    (:`else`
      (bind _returnvalue (`|CreateWidget` "/Game/RoboSupport/UI/Tutorial/WBP_Tutorial_Puzzle.WBP_Tutorial_Puzzle_C"))
      (bind _output_get (set `self.ActivWidget` _returnvalue))
      (`UserWidget.AddToViewport` _output_get 0)
      (set `PlayerController.bShowMouseCursor` true (`GameplayStatics.GetPlayerController` 0)))))

(fn `AddCart`
  (params (Interactor :type "Actor Object Reference"))
  (returns (NewParam :type Boolean))
  (return false))

(fn `GetInteractableActions`
  (returns (Actions :type "Map of /Game/RoboSupport/Inventory/E_Tools Enum to String") (PuzzleRef :type "Actor Object Reference"))
  (return _ null))

(fn `GetInteractableType`
  (returns (NewParam :type "/Game/RoboSupport/Objects/E_InteractType Enum"))
  (return "NewEnumerator0"))

(fn `PuzzleInteract`
  (params (AnyTextIn :type String))
  (returns (AnyTextOut :type String))
  (return ""))

(fn `UserConstructionScript`
  (`WidgetComponent.SetDrawSize` (`self.Widget`) (`self.Size`)))