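; BP_Test_objact is a test actor in RoboSupport that responds to an Interact event by rotating itself 45 degrees in local yaw.
; A ChaosDestructionListener component passes collision events to a sort by highest mass, with nothing acting on the result.
; BeginPlay, overlap and Tick are disabled stubs, the construction script only calls its parent, and a stray Interact call with tool and button inputs never runs.
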(event `/Game/RoboSupport/Interface/BPI_Interact.Interact`
  (params (Interactor :type "Actor Object Reference") (CurrentTool :type "/Game/RoboSupport/Inventory/E_Tools Enum" :default "NewEnumerator4") (PbutoonAct :type "/Game/RoboSupport/Puzzle/E_ElemPButtonAct Enum" :default "NewEnumerator0"))
  (`self.K2_AddActorLocalRotation` (`KismetMathLibrary.MakeRotator` 0.0 0.0 45.0)))

(event `self.ChaosDestructionListener.OnCollisionEvents`
  (params (CollisionEvents :type "Array of ChaosCollisionEventData Structure (by ref)"))
  (`ChaosDestructionListener.SortCollisionEvents` (`self.ChaosDestructionListener`) CollisionEvents "SortByHighestMass"))

(fn `UserConstructionScript`
  (`parent.UserConstructionScript`))