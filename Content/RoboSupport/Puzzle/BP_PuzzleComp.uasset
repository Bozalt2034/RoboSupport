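; Interactive PC repair puzzle actor with clickable supply unit, motherboard and power button, each given an attached particle effect.
; Clicking a part passes its action list to the UI-on-click call.
; PuzzleElemInteract maps the chosen action to a problem status update, with side effects like battery discharge on power-on or fire and explosion sound on RAM installation, then broadcasts OnUpdateState.
; A helper function toggles a test action widget at the mouse cursor.
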(event `self.FixProblem`
  (params (Index :type Integer) (Status :type Boolean))
  (bind _problems (`self.Problems`))
  (`KismetArrayLibrary.Array_Set` _problems Index (make `/Game/RoboSupport/Puzzle/F_defects` (`.Name_10_7756C5F44B5E7448E29089A55EF04FFC` (break `/Game/RoboSupport/Puzzle/F_defects` (`|GetArrayItem` _problems Index))) Status)))

(event `self.SupplyUnit.OnClicked`
  (params (TouchedComponent :type "PrimitiveComponent Object Reference") (ButtonPressed :type "Key Structure"))
  ;[1 1 1] Вызов UI при нажатии на элемент и заполнение UI из массива ENUM
  (`self.CallUIOnClickElem` (`self.ActionSupplyUnit`)))

(event `self.ReceiveBeginPlay`
  (`parent.ReceiveBeginPlay`)
  (bind _returnvalue (`GameplayStatics.SpawnEmitterAttached` (`self.ET_SupplyUnit`) (`self.SupplyUnit`)))
  (set `self.SupplyUnitEffects` _returnvalue)
  (bind _returnvalue_2 (`GameplayStatics.SpawnEmitterAttached` (`self.ET_Motherboard`) (`self.MotherBoard`)))
  (set `self.MotherboardEffects` _returnvalue_2)
  (bind _returnvalue_3 (`GameplayStatics.SpawnEmitterAttached` (`self.ET_PowerButton`) (`self.PowerButton`)))
  (set `self.PowerButtonEffects` _returnvalue_3))

(event `self.PowerButton.OnClicked`
  (params (TouchedComponent :type "PrimitiveComponent Object Reference") (ButtonPressed :type "Key Structure"))
  ;[1 1 1] Вызов UI при нажатии на элемент и заполнение UI из массива ENUM
  (`self.CallUIOnClickElem` (`self.ActionPowerButton`)))

(event `self.MotherBoard.OnClicked`
  (params (TouchedComponent :type "PrimitiveComponent Object Reference") (ButtonPressed :type "Key Structure"))
  ;[1 1 1] Вызов UI при нажатии на элемент и заполнение UI из массива ENUM
  (`self.CallUIOnClickElem` (`self.ActionMoterboard`)))

(event `Testword`
  (`KismetSystemLibrary.PrintString` "click" true true (struct :`R` 1.0 :`A` 1.0)))

(event `OnClicked_Event_0`
  ;[1 1 1] Попытка вызвать клик по кнопке интерфейса
)

(event `/Game/RoboSupport/Interface/BPI_Interact.PuzzleElemInteract`
  (params (Interactor :type "Actor Object Reference") (PbutoonAct :type "/Game/RoboSupport/Puzzle/E_ElemPButtonAct Enum" :default "NewEnumerator0"))
  (bind _problemstatus_replace_cpu_cooler (`self.ProblemStatus:Replace CPU cooler`))
  (bind _motherboardeffects (`self.MotherboardEffects`))
  (bind _problemstatus_add_ram (`self.ProblemStatus:Add RAM`))
  (`|ExecutionSequence`
    (:`then_0`
      (switch `/Game/RoboSupport/Puzzle/E_ElemPButtonAct` PbutoonAct
        (:`NewEnumerator0`
          (`self.FixProblem2` 0 (`self.ProblemStatus:Power On`))
          (`self.Discharge Battery` 5.0)
          (`/Engine/EditorBlueprintResources/StandardMacros.DoOnce` false :!label _label
            (:`Completed`
              (`GameplayStatics.SpawnSound2D` "/Game/RoboSupport/Puzzle/Audio/PC_OnSound.PC_OnSound" 1.0 1.0 0.0 null))))
        (:`NewEnumerator1`
          (`self.FixProblem2` 0 (`self.ProblemStatus:Power Off`))
          (goto _label :!via `Reset`))
        (:`NewEnumerator3`
          (`self.FixProblem2` 0 (`self.ProblemStatus:Unplug AC Cable`)))
        (:`NewEnumerator4`
          (`self.FixProblem2` 0 (`self.ProblemStatus:Plug AC Cable`)))
        (:`NewEnumerator5`
          (`self.FixProblem2` 0 (`self.ProblemStatus:Replace Supply unit`)))
        (:`NewEnumerator6`
          (`self.FixProblem2` 0 (`self.ProblemStatus:Replace Motherboard`)))
        (:`NewEnumerator7`
          (`self.FixProblem2` 0 _problemstatus_replace_cpu_cooler)
          (if (not _problemstatus_replace_cpu_cooler)
            ;[1 1 1] Уничтожит emitter елемент
            (`ActorComponent.K2_DestroyComponent` _motherboardeffects)
            ;[1 1 1] Убрать звуковые эфекты
            (bind _actorsound (`self.ActorSound`)
              (:`then`
                (`AudioComponent.SetSound` _actorsound null))
              (:`else`))))
        (:`NewEnumerator8`
          (`self.FixProblem2` 0 _problemstatus_add_ram)
          (if _problemstatus_add_ram
            (bind _returnvalue (`GameplayStatics.SpawnEmitterAttached` "/Game/Downloads/StarterContent/Particles/P_Fire.P_Fire" _motherboardeffects))
            (set `self.MotherboardEffects` _returnvalue)
            ;[1 1 1] Заспавнить звук в локации актора и записать его в переменную
            (bind _returnvalue_2 (`GameplayStatics.SpawnSoundAtLocation` "/Game/Downloads/StarterContent/Audio/Explosion_Cue.Explosion_Cue" (`self.K2_GetActorLocation`) (struct) 1.0 1.0 0.0 null null))
            (set `self.ActorSound` _returnvalue_2)))))
    (:`then_1`
      (`self.OnUpdateState` self))))

(fn `NewFunction_0_0`
  (params (Array :type "Array of /Game/RoboSupport/Puzzle/E_ElemPButtonAct Enum (by ref)"))
  (bind (_locationx _locationy) (`PlayerController.GetMousePosition` (`GameplayStatics.GetPlayerController` 0)))
  (bind _testui (`self.TestUI`)
    (:`then`
      (`Widget.RemoveFromParent` _testui)
      (set `self.TestUI` null))
    (:`else`
      (bind _returnvalue (`|CreateWidget` "/Game/RoboSupport/Puzzle/Widget/WBP_test.WBP_test_C" null self))
      (bind _output_get (set `self.TestUI` _returnvalue))
      (`UserWidget.AddToViewport` _output_get 0)
      (`/Game/RoboSupport/Puzzle/Widget/WBP_test.FillData` (`self.TestUI`) Array)
      ;[1 1 1] Вызов виджета рядом с курсором мышки
      (`UserWidget.SetPositionInViewport` (`self.TestUI`) (`KismetMathLibrary.MakeVector2D` _locationx _locationy) true))))

(fn `UserConstructionScript`
  (`parent.UserConstructionScript`))