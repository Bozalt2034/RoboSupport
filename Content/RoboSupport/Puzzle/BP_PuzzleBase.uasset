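; Base puzzle actor for the robot-support game: an interactable device with a defect list, action list and countdown timer.
; Exit returns camera and input to the interactor; the code for entering puzzle view is unconnected.
; Hovering elements toggles custom-depth highlights, and CallUIOnClickElem toggles a popup at the cursor.
; FixProblem2 edits defects and refreshes the bobbing indicator, whose visibility follows the last entry; DischargeBattery drains the player robot.
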(event `Exit`
  (bind _returnvalue (`GameplayStatics.GetPlayerController` 0))
  ;[1 0 0] Ошибка. Не возвращается корректное управление камерой
  ;;[1 1 1] Переключение режима игры на персонажа
  ;;;[1 1 1] Переключение камеры на персонажа
  (`PlayerController.SetViewTargetWithBlend` (`GameplayStatics.GetPlayerController` 0) (`self.Interactor`) 0.0 "VTBlend_Linear" 0.0 false)
  ;;;[1 1 1] Remove Puzzle UI
  (bind _asbp_robot_support (cast `/Game/RoboSupport/Characters/BP_RobotSupport` (`self.Interactor`)))
  (`/Game/RoboSupport/Characters/BP_RobotSupport.CreatePuzzleUi` _asbp_robot_support (`self.Actions`) null null)
  ;;;[1 1 1] Отключение ивентов клик и наведение курсора
  (set `PlayerController.bEnableClickEvents` false _returnvalue)
  (set `PlayerController.bEnableMouseOverEvents` false _returnvalue)
  ;;;[1 1 1] Переключение инпутов к обычным
  (`Controller.SetIgnoreLookInput` _returnvalue false)
  (`Controller.SetIgnoreMoveInput` _returnvalue false)
  (set `PlayerController.bShowMouseCursor` false _returnvalue))

(event `/Game/RoboSupport/Interface/BPI_Interact.SetInteractor`
  (params (InNewInteractor :type "Actor Object Reference"))
  (set `self.Interactor` InNewInteractor))

(event `/Game/RoboSupport/Interface/BPI_Interact.Interact`
  (params (Interactor :type "Actor Object Reference") (CurrentTool :type "/Game/RoboSupport/Inventory/E_Tools Enum" :default "NewEnumerator4") (PbutoonAct :type "/Game/RoboSupport/Puzzle/E_ElemPButtonAct Enum" :default "NewEnumerator0"))
  (`|ExecutionSequence`
    (:`then_0`
      (switch `/Game/RoboSupport/Inventory/E_Tools` CurrentTool
        (:`NewEnumerator5`
          (`self.Exit`)
          (bind _elemui (`self.ElemUI`)
            (:`then`
              (`Widget.RemoveFromParent` _elemui)
              (set `self.ElemUI` null))
            (:`else`)))))))

(event `FixProblem`
  (params (Index :type Integer) (Status :type Boolean))
  (bind _problems (`self.Problems`))
  ;[1 1 1] Попытка сделать взаимодействие с списком неисправностей, работает но не достаточно гибко. Использую функцию FixProblem2
  (`KismetArrayLibrary.Array_Set` _problems Index (make `/Game/RoboSupport/Puzzle/F_defects` (`.Name_10_7756C5F44B5E7448E29089A55EF04FFC` (break `/Game/RoboSupport/Puzzle/F_defects` (`|GetArrayItem` _problems Index))) Status)))

(event `self.PuzzleElem.OnBeginCursorOver`
  (params (TouchedComponent :type "PrimitiveComponent Object Reference"))
  (`PrimitiveComponent.SetRenderCustomDepth` TouchedComponent true))

(event `self.ReceiveTick`
  (params (DeltaSeconds :type "Float (single-precision)"))
  ;[1 1 1] Таймер
  ;;[1 1 1] Секунды
  (bind _output_get (set `self.CurrentSecond` (`KismetMathLibrary.FInterpTo_Constant` (`self.CurrentSecond`) (`self.TargetSecond`) DeltaSeconds 1.0)))
  ;;[1 1 1] Проверка счетчика
  (if (== (`self.CurrentSecond`) 0.0)
    ;;[1 1 1] Уменьшение минут, сброс секунд
    (set `self.Minutes` (- (`self.Minutes`) 1))
    (set `self.CurrentSecond` 60.0)))

(event `self.PuzzleElem.OnEndCursorOver`
  (params (TouchedComponent :type "PrimitiveComponent Object Reference"))
  (`PrimitiveComponent.SetRenderCustomDepth` TouchedComponent false))

(event `self.ReceiveBeginPlay`
  (`|ExecutionSequence`
    (:`then_0`
      ;[1 1 1] Спавн звукового эфекта и запись его в переменную
      (bind _returnvalue (`GameplayStatics.SpawnSoundAtLocation` (`self.Sound`) (`self.K2_GetActorLocation`) (struct) 1.0 1.0 0.0 null null))
      (set `self.ActorSound` _returnvalue))
    (:`then_1`
      ;[1 1 1] Анимация индикатора проблемы
      (`self.DefectStatusUpDown`))
    (:`then_2`
      ;[1 1 1] Влючение отображения индикатора проблемы, если есть проблема
      (`self.ProblemIndicator`))))

(event `DefectStatusUpDown`
  ;[1 1 1] Анимация движения индикатора дефекта
  (`/Engine/EditorBlueprintResources/StandardMacros.FlipFlop` :!label _label
    (:`A`
      (bind (_direction _down) (`Timeline|UPnDown` :!label _label_2)
        (:`Update`
          (`SceneComponent.K2_SetRelativeLocation` (`self.DeffectSstatus`) (`KismetMathLibrary.MakeVector` 0.0 0.0 _down) false false)
          (`KismetSystemLibrary.RetriggerableDelay` 0.2)
          (goto _label))))
    (:`B`
      (goto _label_2 :!via `Reverse`))))

(fn `AddCart`
  (params (Interactor :type "Actor Object Reference"))
  (returns (NewParam :type Boolean))
  (return false))

(fn `CallUIOnClickElem`
  (params (Array :type "Array of /Game/RoboSupport/Puzzle/E_ElemPButtonAct Enum (by ref)"))
  (bind (_locationx _locationy) (`PlayerController.GetMousePosition` (`GameplayStatics.GetPlayerController` 0)))
  (bind _elemui (`self.ElemUI`)
    (:`then`
      (`Widget.RemoveFromParent` _elemui)
      (set `self.ElemUI` null))
    (:`else`
      (bind _returnvalue (`|CreateWidget` "/Game/RoboSupport/Puzzle/Widget/WBP_test.WBP_test_C" null self))
      (bind _output_get (set `self.ElemUI` _returnvalue))
      (`UserWidget.AddToViewport` _output_get 0)
      (`/Game/RoboSupport/Puzzle/Widget/WBP_test.FillData` (`self.ElemUI`) Array)
      ;[1 1 1] Вызов виджета рядом с курсором мышки
      (`UserWidget.SetPositionInViewport` (`self.ElemUI`) (`KismetMathLibrary.MakeVector2D` _locationx _locationy) true))))

(fn `Discharge Battery`
  (params (Discharge :type "Float (double-precision)"))
  (bind _asbp_robot_support (cast `/Game/RoboSupport/Characters/BP_RobotSupport` (`GameplayStatics.GetPlayerPawn` 0)))
  (`/Game/RoboSupport/Characters/BP_RobotSupport.Battery Disсharge` _asbp_robot_support Discharge))

(fn `FixProblem2`
  (params (Index :type Integer) (Status :type Boolean))
  (`KismetArrayLibrary.Array_Set` (`self.Problems`) 0 (make `/Game/RoboSupport/Puzzle/F_defects` (`.Name_10_7756C5F44B5E7448E29089A55EF04FFC` (break `/Game/RoboSupport/Puzzle/F_defects` (`|GetArrayItem` (`self.Problems`) Index))) Status))
  (`self.ProblemIndicator`))

(fn `GetInteractableActions`
  (returns (Actions :type "Map of /Game/RoboSupport/Inventory/E_Tools Enum to String") (PuzzleRef :type "Actor Object Reference"))
  (return (`self.Actions`) self))

(fn `GetInteractableType`
  (returns (NewParam :type "/Game/RoboSupport/Objects/E_InteractType Enum"))
  (return "NewEnumerator1"))

(fn `ProblemIndicator`
  ;[1 1 1] Отображение индикатора проблемы, если есть проблема
  (for _array_element (`self.Problems`)
    (`SceneComponent.SetVisibility` (`self.DeffectSstatus`) (`.DefectStatus_13_60C5A6DB492FFE0DB8E3EB9B40C85E32` (break `/Game/RoboSupport/Puzzle/F_defects` _array_element)) false)))

(fn `PuzzleInteract`
  (params (AnyTextIn :type String))
  (returns (AnyTextOut :type String))
  (`KismetSystemLibrary.PrintString` AnyTextIn)
  (return ""))

(fn `UserConstructionScript`)