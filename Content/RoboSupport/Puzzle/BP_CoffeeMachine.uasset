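; Coffee machine puzzle actor with clickable buttons to add coffee, cola and energy drink, plus a start button.
; Each ingredient button sets a flag and switches once to a glow material.
; The first Start press spawns the matching drink only if coffee was added, then shows DoneStatus and calls FixProblem2.
; A DoOnce consumes that press even without coffee, while OnUpdateState is called on every press.
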(event `self.StartButton.OnClicked`
  (params (TouchedComponent :type "PrimitiveComponent Object Reference") (ButtonPressed :type "Key Structure"))
  (`|ExecutionSequence`
    (:`then_0`
      (`/Engine/EditorBlueprintResources/StandardMacros.DoOnce` false
        (:`Completed`
          (if (`self.AddedCoffee`)
            (if (or (`self.AddedCola`) (`self.AddedEnergyDrink`))
              (if (and (`self.AddedCoffee`) (`self.AddedCola`) (`self.AddedEnergyDrink`))
                (`|SpawnActorFromClass` "/Game/RoboSupport/Inventory/Items/BP_Coffee+Cola+ED.BP_Coffee+Cola+ED_C" (`self.GetTransform` (`self.SpawnPoint`)) "Undefined" "OverrideRootScale" null null)
                (`SceneComponent.SetVisibility` (`self.DoneStatus`) true false :!label _label)
                (`self.FixProblem2` 0)
                (elif (and (`self.AddedCoffee`) (`self.AddedCola`))
                  (`|SpawnActorFromClass` "/Game/RoboSupport/Inventory/Items/BP_Coffee+Cola.BP_Coffee+Cola_C" (`self.GetTransform` (`self.SpawnPoint`)) "Undefined" "OverrideRootScale" null null)
                  (goto _label)
                  (elif (and (`self.AddedCoffee`) (`self.AddedEnergyDrink`))
                    (`|SpawnActorFromClass` "/Game/RoboSupport/Inventory/Items/BP_Coffee+ED.BP_Coffee+ED_C" (`self.GetTransform` (`self.SpawnPoint`)) "Undefined" "OverrideRootScale" null null)
                    (goto _label))))
              (else
                (`|SpawnActorFromClass` "/Game/RoboSupport/Inventory/Items/BP_coffee.BP_coffee_C" (`self.GetTransform` (`self.SpawnPoint`)) "Undefined" "OverrideRootScale" null null)
                (goto _label)))))))
    (:`then_1`
      (`self.OnUpdateState` self))))

(event `self.AddCoffee.OnClicked`
  (params (TouchedComponent :type "PrimitiveComponent Object Reference") (ButtonPressed :type "Key Structure"))
  (set `self.AddedCoffee` true)
  (`/Engine/EditorBlueprintResources/StandardMacros.DoOnce` false
    (:`Completed`
      (`PrimitiveComponent.SetMaterial` (`self.AddCoffee`) 0 "/Game/RoboSupport/Material/M_GreenGlow_Inst1.M_GreenGlow_Inst1"))))

(event `self.AddEnergyDrink.OnClicked`
  (params (TouchedComponent :type "PrimitiveComponent Object Reference") (ButtonPressed :type "Key Structure"))
  (set `self.AddedEnergyDrink` true)
  (`/Engine/EditorBlueprintResources/StandardMacros.DoOnce` false
    (:`Completed`
      (`PrimitiveComponent.SetMaterial` (`self.AddEnergyDrink`) 0 "/Game/RoboSupport/Material/M_BlueGlow_Inst.M_BlueGlow_Inst"))))

(event `self.AddCola.OnClicked`
  (params (TouchedComponent :type "PrimitiveComponent Object Reference") (ButtonPressed :type "Key Structure"))
  (set `self.AddedCola` true)
  (`/Engine/EditorBlueprintResources/StandardMacros.DoOnce` false
    (:`Completed`
      (`PrimitiveComponent.SetMaterial` (`self.AddCola`) 0 "/Game/RoboSupport/Material/M_YellowGlow_Inst.M_YellowGlow_Inst"))))

(fn `UserConstructionScript`
  (`parent.UserConstructionScript`))