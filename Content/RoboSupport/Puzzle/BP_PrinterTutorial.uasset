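; Tutorial printer puzzle element, built on a parent class, with clickable parts that each send their action list to the UI.
; The Add Paper action calls FixProblem2, drains battery and adds an item to the robot pawn's inventory; every interaction then broadcasts a state update.
; DefectStatusUpDown bobs the defect status component vertically, using a timeline, FlipFlop and retriggerable delay to reverse direction once updates stop.
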(event `self.DefectStatusUpDown`
  (`/Engine/EditorBlueprintResources/StandardMacros.FlipFlop` :!label _label
    (:`A`
      (bind (_direction _down) (`Timeline|UpNDownPrinter` :!label _label_2)
        (:`Update`
          (`SceneComponent.K2_SetRelativeLocation` (`self.DeffectSstatus`) (`KismetMathLibrary.MakeVector` 0.0 0.0 _down) false false)
          (`KismetSystemLibrary.RetriggerableDelay` 0.2)
          (goto _label))))
    (:`B`
      (goto _label_2 :!via `Reverse`))))

(event `self.ReceiveBeginPlay`
  (`parent.ReceiveBeginPlay`))

(event `/Game/RoboSupport/Interface/BPI_Interact.PuzzleElemInteract`
  (params (Interactor :type "Actor Object Reference") (PbutoonAct :type "/Game/RoboSupport/Puzzle/E_ElemPButtonAct Enum" :default "NewEnumerator0"))
  (`|ExecutionSequence`
    (:`then_0`
      (switch `/Game/RoboSupport/Puzzle/E_ElemPButtonAct` PbutoonAct
        (:`NewEnumerator9`
          (`self.FixProblem2` 0)
          (`self.Discharge Battery` 10.0)
          (bind _asbp_robot_support (cast `/Game/RoboSupport/Characters/BP_RobotSupport` (`GameplayStatics.GetPlayerPawn` 0)))
          (`/Game/RoboSupport/Inventory/AC_InventoriComponent.AddItem` (`/Game/RoboSupport/Characters/BP_RobotSupport.BPC_InventoriComponent` _asbp_robot_support) (`self.To Add`)))))
    (:`then_1`
      (`self.OnUpdateState` self))))

(event `self.Cartridge.OnClicked`
  (params (TouchedComponent :type "PrimitiveComponent Object Reference") (ButtonPressed :type "Key Structure"))
  ;[1 1 1] Заполнение виджета нажатия действиями
  (`self.CallUIOnClickElem` (`self.ActionsCartridge`)))

(event `self.PrinterComponents.OnClicked`
  (params (TouchedComponent :type "PrimitiveComponent Object Reference") (ButtonPressed :type "Key Structure"))
  ;[1 1 1] Заполнение виджета нажатия действиями
  (`self.CallUIOnClickElem` (`self.ActionsPrinterComponents`)))

(event `self.PaperCassette.OnClicked`
  (params (TouchedComponent :type "PrimitiveComponent Object Reference") (ButtonPressed :type "Key Structure"))
  ;[1 1 1] Заполнение виджета нажатия действиями
  (`self.CallUIOnClickElem` (`self.ActionsPaperCassette`)))

(event `self.On/Off_Switch.OnClicked`
  (params (TouchedComponent :type "PrimitiveComponent Object Reference") (ButtonPressed :type "Key Structure"))
  ;[1 1 1] Заполнение виджета нажатия действиями
  (`self.CallUIOnClickElem` (`self.ActionsOn/Off_switch`)))

(fn `UserConstructionScript`
  (`parent.UserConstructionScript`))